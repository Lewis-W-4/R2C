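; BP_HexGrid builds a hex tile grid with randomised heights in its construction script.
; Nested loops add GridTiles instances, shifting odd columns by Offset and using a random Elevation for Z position and scale.
; Each cell also gets a small Points instance at ten times that elevation.
; Colours sets BasicUnit on material slot 1 of the whole GridTiles component when Elevation reaches a threshold, so it is not per tile.
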(event EventBeginPlay)

(event Collision|EventActorBeginOverlap
  (params (OtherActor :type Actor%20Object%20Reference)))

(event EventTick
  (params (DeltaSeconds :type Float%20%28single-precision%29)))

(fn ConstructionScript
  (Components|StaticMesh|SetStaticMesh (Variables|Default|GetGridTiles) (Variables|Default|GetTileMesh))
  (for _index (range 0 (Variables|Default|GetGrid%20X))
    (for _index_2 (range 0 (Variables|Default|GetGrid%20Y))
      (Variables|Default|SetElevation (Math|Random|RandomFloatinRange 1.0 7.0))
      (Components|InstancedStaticMesh|AddInstance (Variables|Default|GetGridTiles) (Math|Transform|MakeTransform (Math|Vector|MakeVector (.x (Math|Vector|SelectVector (Math|Vector|MakeVector (* _index (Variables|Default|GetSpacing%20X)) (* _index_2 (Variables|Default|GetSpacing%20Y)) 0.0) (Math|Vector|MakeVector (* _index (Variables|Default|GetSpacing%20X)) (+ (Variables|Default|GetOffset) (* _index_2 (Variables|Default|GetSpacing%20Y))) 0.0) (== (Math|Integer|%(Integer) _index 2) 0))) (.y (Math|Vector|SelectVector (Math|Vector|MakeVector (* _index (Variables|Default|GetSpacing%20X)) (* _index_2 (Variables|Default|GetSpacing%20Y)) 0.0) (Math|Vector|MakeVector (* _index (Variables|Default|GetSpacing%20X)) (+ (Variables|Default|GetOffset) (* _index_2 (Variables|Default|GetSpacing%20Y))) 0.0) (== (Math|Integer|%(Integer) _index 2) 0))) (Variables|Default|GetElevation)) "0, 0, 0" (Math|Vector|MakeVector 2.0 2.0 (Variables|Default|GetElevation))))
      (CallFunction|Colours)
      (Components|InstancedStaticMesh|AddInstance (Variables|Default|GetPoints) (Math|Transform|MakeTransform (Math|Vector|MakeVector (.x (Math|Vector|SelectVector (Math|Vector|MakeVector (* _index (Variables|Default|GetSpacing%20X)) (* _index_2 (Variables|Default|GetSpacing%20Y)) 0.0) (Math|Vector|MakeVector (* _index (Variables|Default|GetSpacing%20X)) (+ (Variables|Default|GetOffset) (* _index_2 (Variables|Default|GetSpacing%20Y))) 0.0) (== (Math|Integer|%(Integer) _index 2) 0))) (.y (Math|Vector|SelectVector (Math|Vector|MakeVector (* _index (Variables|Default|GetSpacing%20X)) (* _index_2 (Variables|Default|GetSpacing%20Y)) 0.0) (Math|Vector|MakeVector (* _index (Variables|Default|GetSpacing%20X)) (+ (Variables|Default|GetOffset) (* _index_2 (Variables|Default|GetSpacing%20Y))) 0.0) (== (Math|Integer|%(Integer) _index 2) 0))) (* (Variables|Default|GetElevation) 1e+01)) "0, 0, 0" (Math|Vector|MakeVector 0.5 0.5 0.5))))))

(fn Colours
  (if (>= (Variables|Default|GetElevation) 4.0)
    (Rendering|Material|SetMaterial (Variables|Default|GetGridTiles) 1 "/Game/Units/UnitColours/BasicUnit.BasicUnit")))