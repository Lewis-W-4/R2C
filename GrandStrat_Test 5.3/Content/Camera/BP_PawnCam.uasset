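; BP_PawnCam is a camera Blueprint that provides mouse-wheel zoom and puts the construction HUD on screen.
; Wheel up and down shorten or lengthen the SpringArm in fixed steps, skipping any step that would pass the minimum or maximum arm length.
; On BeginPlay it creates a Construction_HUD widget, stores it in HUD and adds it to the viewport.
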(event EventBeginPlay
  ;[1 1 1] HUD - Set Up
  (bind _returnvalue (UserInterface|CreateWidget "/Game/HUD/Construction_HUD/Construction_HUD.Construction_HUD_C"))
  (bind _output_get (Variables|Default|SetHUD _returnvalue))
  (UserInterface|Viewport|AddtoViewport _output_get 0))

(event Input|MouseEvents|MouseWheelUp
  (params (Key :type Key%20Structure))
  (bind _springarm (Variables|Default|GetSpringArm))
  ;[1 1 1] Mouse Scrolling - Zoom In
  (:Pressed
    (if (>= (- (Variables|/Script/Engine.SpringArmComponent|GetTargetArmLength _springarm) 5e+01) 1.0)
      (Variables|/Script/Engine.SpringArmComponent|SetTargetArmLength _springarm (- (Variables|/Script/Engine.SpringArmComponent|GetTargetArmLength _springarm) 5e+01)))))

(event Input|MouseEvents|MouseWheelDown
  (params (Key :type Key%20Structure))
  (bind _springarm (Variables|Default|GetSpringArm))
  ;[1 1 1] Mouse Scrolling - Zoom Out
  (:Pressed
    (if (<= (+ (Variables|/Script/Engine.SpringArmComponent|GetTargetArmLength _springarm) 5e+01) 1.75e+03)
      (Variables|/Script/Engine.SpringArmComponent|SetTargetArmLength _springarm (+ (Variables|/Script/Engine.SpringArmComponent|GetTargetArmLength _springarm) 5e+01)))))

(fn ConstructionScript)