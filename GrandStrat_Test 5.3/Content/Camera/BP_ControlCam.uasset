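; Player controller that drives the BP_PawnCam camera and handles mouse-based building placement, which starts enabled at BeginPlay.
; The camera pans by screen-edge scrolling and by move axes, with axis speed scaled by clamped spring arm length.
; Placement mode spawns a preview actor that follows a cursor line trace each tick.
; The Building input spawns the real building when the preview's BP_Plop reports valid placement, then exits the mode.
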(event EventBeginPlay
  (Utilities|Camera)
  (Variables|Default|SetbShowMouseCursor true)
  (CallFunction|SetPlacementModeEnabled true))

(event EventTick
  (params (DeltaSeconds :type Float%20%28single-precision%29))
  (if (Variables|Default|GetPlacementModeEnabled)
    (CallFunction|UpdatePlacement)))

(event Input|ActionEvents|InputActionBuilding
  (params (Key :type Key%20Structure :default "None"))
  (:Pressed
    (if (Variables|Default|GetPlacementModeEnabled)
      (CallFunction|SpawnBuilding))))

(event Input|AxisEvents|InputAxisXMove
  (params (AxisValue :type Float%20%28single-precision%29))
  (bind _campawnref (Variables|Default|GetCamPawnRef))
  ;[1 1 1] Moving Along (Left + Right)
  (Transformation|SetActorTransform _campawnref (Utilities|MovementY AxisValue (CallFunction|MovementSpeedCalc) (Variables|Default|GetMoveSens) _campawnref)))

(event Input|AxisEvents|InputAxisYMove
  (params (AxisValue :type Float%20%28single-precision%29))
  (bind _campawnref (Variables|Default|GetCamPawnRef))
  ;[1 1 1] Moving Along (Up + Down)
  (Transformation|SetActorTransform _campawnref (Utilities|MovementX AxisValue (CallFunction|MovementSpeedCalc) (Variables|Default|GetMoveSens) _campawnref)))

(event Input|MouseEvents|MouseX
  (params (AxisValue :type Float%20%28single-precision%29))
  ;[1 1 1] Move Camera With Mouse
  (bind (_delta_xs _delta_ys) (Utilities|ScreenMovement)
    (:Return
      (Transformation|AddActorLocalOffset (Variables|Default|GetCamPawnRef) (Math|Vector|MakeVector _delta_xs _delta_ys 0.0) false false))))

(event Input|MouseEvents|MouseY
  (params (AxisValue :type Float%20%28single-precision%29))
  ;[1 1 1] Move Camera With Mouse
  (Utilities|ScreenMovement) ; enters at Mouse Y
)

(fn ConstructionScript)

(fn MovementSpeedCalc
  (return (Math|Float|Clamp(Float) (/ (Variables|/Script/Engine.SpringArmComponent|GetTargetArmLength (Variables|/Game/Camera/BP_PawnCam.BP_PawnCam_C|GetSpringArm (Variables|Default|GetCamPawnRef))) 1e+02) 5.0 2e+01)))

(fn SetPlacementModeEnabled
  (params (IsEnabled :type Boolean))
  (if (== IsEnabled (Variables|Default|GetPlacementModeEnabled))
    (return)
    (else
      (bind _output_get (Variables|Default|SetPlacementModeEnabled IsEnabled))
      (if _output_get
        (bind _returnvalue (Game|SpawnActorfromClass (Variables|Default|GetPlaceableActorClass) (Math|Transform|MakeTransform "0.000000,0.000000,-100000.000000") "AlwaysSpawn" "MultiplyWithRoot" 0 0))
        (bind _output_get_2 (Variables|Default|SetPlaceableActor _returnvalue))
        (Utilities|IsValid (Actor|GetComponentbyClass _output_get_2 "/Game/Construction/BP_Clickable.BP_Clickable_C")
          (:Is%20Not%20Valid
            (AddComponent|AddBPPlop _output_get_2)))
        (else
          (Utilities|IsValid (Variables|Default|GetPlaceableActor)
            (:Is%20Valid
              (Actor|DestroyActor (Variables|Default|GetPlaceableActor)))))))))

(fn UpdatePlacement
  (bind (_worldlocation _worlddirection) (Game|Player|ConvertMouseLocationToWorldSpace))
  (bind _outhit (Collision|LineTraceByChannel _worldlocation (+ _worlddirection (* _worlddirection 1e+04)) "TraceTypeQuery3" false 0 "None"))
  (if (.bBlockingHit (Collision|BreakHitResult _outhit))
    (Transformation|SetActorLocation (Variables|Default|GetPlaceableActor) (.Location (Collision|BreakHitResult _outhit)) false false)))

(fn SpawnBuilding
  (bind _placeableactor (Variables|Default|GetPlaceableActor))
  (bind _returnvalue (Actor|GetComponentbyClass _placeableactor "/Game/Construction/BP_Plop.BP_Plop_C"))
  (Utilities|IsValid _returnvalue
    (:Is%20Valid
      (if (Variables|/Game/Construction/BP_Plop.BP_Plop_C|GetIsPlacementValid _returnvalue)
        (Game|SpawnActorfromClass (Variables|Default|GetPlaceableActorClass) (Transformation|GetActorTransform (Variables|Default|GetPlaceableActor)) "AlwaysSpawn" "MultiplyWithRoot" 0 0)
        (CallFunction|SetPlacementModeEnabled false)))))