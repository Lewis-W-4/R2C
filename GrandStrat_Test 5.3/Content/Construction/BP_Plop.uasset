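; BP_Plop is a construction component that shows whether its owning actor sits in a valid, unobstructed spot.
; It binds to the owner's begin and end overlap events, rechecking on each and at BeginPlay; any overlapping actor makes placement invalid.
; Each check swaps the first material slot of all the owner's static meshes between valid and invalid plop materials.
; The InPlacementMode event destroys the component.
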(event Custom|OverlapState
  (params (OverlappedActor :type Actor%20Object%20Reference) (OtherActor :type Actor%20Object%20Reference))
  (CallFunction|UpdateState))

(event Custom|InPlacementMode
  (Components|DestroyComponent))

(event EventBeginPlay
  (bind _returnvalue (Components|GetOwner))
  (Collision|BindEventtoOnActorBeginOverlap _returnvalue (delegate Custom|OverlapState))
  (Collision|BindEventtoOnActorEndOverlap _returnvalue (delegate Custom|OverlapState))
  (CallFunction|UpdateState))

(fn UpdateState
  (bind _output_get (Variables|Default|SetIsPlacementValid (== (Utilities|Array|Length (Collision|GetOverlappingActors (Components|GetOwner) "/Script/Engine.Actor" :!class /Script/Engine.Actor)) 0)))
  (for _array_element (Actor|GetComponentsByClass (Components|GetOwner) "/Script/Engine.StaticMeshComponent")
    (if _output_get
      (Rendering|Material|SetMaterial _array_element 0 (Variables|Default|GetPlopMat))
      (else
        (Rendering|Material|SetMaterial _array_element 0 (Variables|Default|GetInvalidPlopMat))))))